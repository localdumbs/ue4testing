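; Generator actor that procedurally grows a branching, axis-aligned network of spline walls inside a square area.
; It seeds a grid of WallClass actors with random cardinal directions, then each step kills colliding paths, spawns perpendicular branches, extends paths and stops out-of-bounds ones.
; Generate steps on a looping timer and fires Generated when all paths die, while Run loops synchronously for editor use.
; Clear removes tagged splines; CalculateProbability provides capped, exponential length-based odds.
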(event Custom|Run
  (bind _returnvalue (Transformation|GetActorLocation))
  (bind _returnvalue_2 (Transformation|GetActorLocation))
  (bind _self self)
  (bind _size (Variables|Default|GetSize))
  (bind _size_2 (Variables|Default|GetSize))
  (bind _startingwallsamount (Variables|Default|GetStartingWallsAmount))
  (bind _size_3 (Variables|Default|GetSize))
  (bind _startingwallsamount_2 (Variables|Default|GetStartingWallsAmount))
  (bind _returnvalue_3 (/ _size 2.0))
  (bind _returnvalue_4 (/ _size_3 2.0))
  (bind _returnvalue_5 (+ _startingwallsamount 1))
  (bind _returnvalue_6 (Math|Conversions|ToFloat(Integer) _returnvalue_5))
  (bind _returnvalue_7 (- _returnvalue_2 _returnvalue_4))
  (bind _returnvalue_8 (/ _size_2 _returnvalue_6))
  ;[1 1 1] IN EDITOR
  (for _index (range 0 (- (Math|Float|Truncate (Math|Float|Square (Math|Conversions|ToFloat(Integer) (Variables|Default|GetStartingWallsAmount)))) 1))
    (bind _returnvalue_9 (Game|SpawnActorfromClass (Variables|Default|GetWallClass) (Math|Transform|MakeTransform (+ (Math|Vector|MakeVector (* (+ (Math|Integer|%(Integer) _index _startingwallsamount_2) 1) _returnvalue_8) (* (+ (/ _index _startingwallsamount_2) 1) _returnvalue_8) 0.0) (Math|Vector|MakeVector (.x _returnvalue_7) (.y _returnvalue_7) (.Z (Math|Vector|BreakVector _returnvalue_2)))) "0, 0, 0" "1,1,1") "Undefined" self (Utilities|Select :Index (Math|Float|Floor (* (Math|Random|RandomFloat) 4.0)) :Option%200 "1.000000, 0, 0" :Option%201 "0,1.000000, 0" :Option%202 "-1.000000, 0, 0" :Option%203 "0,-1.000000, 0") (Variables|Default|GetSpline%20Increment%20Amount) 0.0 0))
    (Transformation|SetActorRotation _returnvalue_9 (Math|Conversions|RotationFromXVector (Variables|/Game/BP_WallSpline.BP_WallSpline_C|GetDirectionVector _returnvalue_9)))
    (Utilities|Array|Add (Variables|Default|GetPaths) _returnvalue_9))
  (Variables|Default|SetLoopCount 0)
  (while (not (Variables|Default|GetStop))
    (Math|Integer|IncrementInt (Variables|Default|GetLoopCount)
      (:%20%20
        (Utilities|Array|AppendArray (Variables|Default|GetPaths) (Variables|Default|GetNew%20Paths))
        (Utilities|Array|Clear (Variables|Default|GetNew%20Paths))
        ;[1 1 1] Kill any colliding paths
        (for _array_element (Variables|Default|GetPaths)
          (Utilities|IsValid _array_element
            (:Is%20Valid
              (if (not (Variables|/Game/BP_WallSpline.BP_WallSpline_C|GetDead _array_element))
                (bind (_collide _object) (Default|CheckCollision _array_element (Variables|Default|GetCollisionBoxSize) (Variables|/Game/BP_WallSpline.BP_WallSpline_C|GetParent _array_element)))
                (Utilities|IsValid _object
                  (:Is%20Valid
                    (if (Math|Boolean|ANDBoolean (!= _object (Variables|/Game/BP_WallSpline.BP_WallSpline_C|GetParent _array_element)) (!= (Variables|/Game/BP_WallSpline.BP_WallSpline_C|GetParent _object) _array_element) _collide)
                      (Default|SetDead _object)
                      (Default|SetDead _array_element))))))))
        ;[1 1 1] Spawn new paths
        (for _array_element_2 (Variables|Default|GetPaths)
          (if (== (Math|Integer|%(Integer) (Variables|Default|GetLoopCount) (/ (Variables|Default|GetBranchCheckFrequency) (Math|Float|Truncate (Variables|Default|GetSpline%20Increment%20Amount)))) 0)
            (Utilities|IsValid _array_element_2
              (:Is%20Valid
                (bind _should (Default|ShouldBranch _array_element_2))
                (if _should
                  (if (!= (.x (Variables|/Game/BP_WallSpline.BP_WallSpline_C|GetDirectionVector _array_element_2)) 0.0)
                    (bind _returnvalue_10 (Game|SpawnActorfromClass (Variables|Default|GetWallClass) (Math|Transform|MakeTransform (Default|GetEnd _array_element_2) "0, 0, 0" "1,1,1") "Undefined" _self (Math|Vector|MakeVector 0.0 (Math|Float|SelectFloat 1.0 -1.0 (Math|Random|RandomBool)) 0.0) (Variables|Default|GetSpline%20Increment%20Amount) (Variables|Default|GetMin%20Wall%20Length) 0))
                    (Transformation|SetActorRotation _returnvalue_10 (Math|Conversions|RotationFromXVector (Variables|/Game/BP_WallSpline.BP_WallSpline_C|GetDirectionVector _returnvalue_10)))
                    (Utilities|Array|Add (Variables|Default|GetNew%20Paths) _returnvalue_10)
                    (Variables|/Game/BP_WallSpline.BP_WallSpline_C|SetParent _returnvalue_10 _array_element_2)
                    (else
                      (bind _returnvalue_11 (Game|SpawnActorfromClass (Variables|Default|GetWallClass) (Math|Transform|MakeTransform (Default|GetEnd _array_element_2) "0, 0, 0" "1,1,1") "Undefined" _self (Math|Vector|MakeVector (Math|Float|SelectFloat 1.0 -1.0 (Math|Random|RandomBool)) 0.0 0.0) (Variables|Default|GetSpline%20Increment%20Amount) (Variables|Default|GetMin%20Wall%20Length) 0))
                      (Transformation|SetActorRotation _returnvalue_11 (Math|Conversions|RotationFromXVector (Variables|/Game/BP_WallSpline.BP_WallSpline_C|GetDirectionVector _returnvalue_11)))
                      (Utilities|Array|Add (Variables|Default|GetNew%20Paths) _returnvalue_11)
                      (Variables|/Game/BP_WallSpline.BP_WallSpline_C|SetParent _returnvalue_11 _array_element_2)))
                  (Variables|/Game/BP_WallSpline.BP_WallSpline_C|SetSpawned _array_element_2 true))))))
        ;[1 1 1] Update all paths, and kill any paths exceeding the bounds
        (Variables|Default|SetStop true)
        (for _array_element_3 (Variables|Default|GetPaths)
          (Utilities|IsValid _array_element_3
            (:Is%20Valid
              (Default|Update _array_element_3)
              (if (Math|Boolean|ORBoolean (< (.x (Default|GetEnd _array_element_3)) (- (.x _returnvalue) _returnvalue_3)) (> (.x (Default|GetEnd _array_element_3)) (+ (.x _returnvalue) _returnvalue_3)) (< (.y (Default|GetEnd _array_element_3)) (- (.y _returnvalue) _returnvalue_3)) (> (.y (Default|GetEnd _array_element_3)) (+ (.y _returnvalue) _returnvalue_3)))
                (Default|SetDead _array_element_3)
                (elif (not (Variables|/Game/BP_WallSpline.BP_WallSpline_C|GetDead _array_element_3))
                  (Variables|Default|SetStop false))))))
        ;[1 1 1] If at runtime, send event dispatchers etc.
        (if (Utilities|Time|IsValidTimerHandle (Variables|Default|GetUpdateTimer))
          (if (Variables|Default|GetStop)
            (Utilities|Time|ClearandInvalidateTimerbyHandle (Variables|Default|GetUpdateTimer))
            (Default|CallGenerated)))))))

(event Custom|Generate
  (bind _returnvalue (Transformation|GetActorLocation))
  (bind _size (Variables|Default|GetSize))
  (bind _startingwallsamount (Variables|Default|GetStartingWallsAmount))
  (bind _size_2 (Variables|Default|GetSize))
  (bind _startingwallsamount_2 (Variables|Default|GetStartingWallsAmount))
  (bind _returnvalue_2 (/ _size_2 2.0))
  (bind _returnvalue_3 (+ _startingwallsamount 1))
  (bind _returnvalue_4 (- _returnvalue _returnvalue_2))
  (bind _returnvalue_5 (Math|Conversions|ToFloat(Integer) _returnvalue_3))
  (bind _returnvalue_6 (/ _size _returnvalue_5))
  ;[1 1 1] RUNTIME
  (for _index (range 0 (- (Math|Float|Truncate (Math|Float|Square (Math|Conversions|ToFloat(Integer) (Variables|Default|GetStartingWallsAmount)))) 1))
    (bind _returnvalue_7 (Game|SpawnActorfromClass (Variables|Default|GetWallClass) (Math|Transform|MakeTransform (+ (Math|Vector|MakeVector (* (+ (Math|Integer|%(Integer) _index _startingwallsamount_2) 1) _returnvalue_6) (* (+ (/ _index _startingwallsamount_2) 1) _returnvalue_6) 0.0) (Math|Vector|MakeVector (.x _returnvalue_4) (.y _returnvalue_4) (.Z (Math|Vector|BreakVector _returnvalue)))) "0, 0, 0" "1,1,1") "Undefined" self (Utilities|Select :Index (Math|Float|Floor (* (Math|Random|RandomFloat) 4.0)) :Option%200 "1.000000, 0, 0" :Option%201 "0,1.000000, 0" :Option%202 "-1.000000, 0, 0" :Option%203 "0,-1.000000, 0") (Variables|Default|GetSpline%20Increment%20Amount) (Variables|Default|GetMin%20Wall%20Length) 0))
    (Transformation|SetActorRotation _returnvalue_7 (Math|Conversions|RotationFromXVector (Variables|/Game/BP_WallSpline.BP_WallSpline_C|GetDirectionVector _returnvalue_7)))
    (Utilities|Array|Add (Variables|Default|GetPaths) _returnvalue_7))
  (bind _returnvalue_8 (Utilities|Time|SetTimerbyEvent (delegate Custom|ev) (Variables|Default|GetStability) true))
  (Variables|Default|SetUpdateTimer _returnvalue_8))

(event Custom|Support%20my%20youtube%20here!%20%28click%29
  ;[1 1 1] THANK YOU
  (Utilities|Platform|LaunchURL "https://www.youtube.com/channel/UCVDMniIN08aTihqNgk7Unbw"))

(event Custom|Clear
  ;[1 1 1] IN EDITOR
  (bind _outactors (Actor|GetAllActorsOfClasswithTag "/Game/BP_WallSpline.BP_WallSpline_C" "generated_spline"))
  (for _array_element _outactors
    (Actor|DestroyActor _array_element)))

(event Custom|ev
  (bind _returnvalue (Transformation|GetActorLocation))
  (bind _self self)
  (bind _size (Variables|Default|GetSize))
  (bind _returnvalue_2 (/ _size 2.0))
  ;[1 1 1] RUNTIME
  (Math|Integer|IncrementInt (Variables|Default|GetLoopCount)
    (:%20%20
      (Utilities|Array|AppendArray (Variables|Default|GetPaths) (Variables|Default|GetNew%20Paths))
      (Utilities|Array|Clear (Variables|Default|GetNew%20Paths))
      ;[1 1 1] Kill any colliding paths
      (for _array_element (Variables|Default|GetPaths)
        (Utilities|IsValid _array_element
          (:Is%20Valid
            (if (not (Variables|/Game/BP_WallSpline.BP_WallSpline_C|GetDead _array_element))
              (bind (_collide _object) (Default|CheckCollision _array_element (Variables|Default|GetCollisionBoxSize) (Variables|/Game/BP_WallSpline.BP_WallSpline_C|GetParent _array_element)))
              (Utilities|IsValid _object
                (:Is%20Valid
                  (if (Math|Boolean|ANDBoolean (!= _object (Variables|/Game/BP_WallSpline.BP_WallSpline_C|GetParent _array_element)) (!= (Variables|/Game/BP_WallSpline.BP_WallSpline_C|GetParent _object) _array_element) _collide)
                    (Default|SetDead _object)
                    (Default|SetDead _array_element))))))))
      ;[1 1 1] Spawn new paths
      (for _array_element_2 (Variables|Default|GetPaths)
        (if (== (Math|Integer|%(Integer) (Variables|Default|GetLoopCount) (/ (Variables|Default|GetBranchCheckFrequency) (Math|Float|Truncate (Variables|Default|GetSpline%20Increment%20Amount)))) 0)
          (Utilities|IsValid _array_element_2
            (:Is%20Valid
              (bind _should (Default|ShouldBranch _array_element_2))
              (if _should
                (if (!= (.x (Variables|/Game/BP_WallSpline.BP_WallSpline_C|GetDirectionVector _array_element_2)) 0.0)
                  (bind _returnvalue_3 (Game|SpawnActorfromClass (Variables|Default|GetWallClass) (Math|Transform|MakeTransform (Default|GetEnd _array_element_2) "0, 0, 0" "1,1,1") "Undefined" _self (Math|Vector|MakeVector 0.0 (Math|Float|SelectFloat 1.0 -1.0 (Math|Random|RandomBool)) 0.0) (Variables|Default|GetSpline%20Increment%20Amount) (Variables|Default|GetMin%20Wall%20Length) 0))
                  (Transformation|SetActorRotation _returnvalue_3 (Math|Conversions|RotationFromXVector (Variables|/Game/BP_WallSpline.BP_WallSpline_C|GetDirectionVector _returnvalue_3)))
                  (Utilities|Array|Add (Variables|Default|GetNew%20Paths) _returnvalue_3)
                  (Variables|/Game/BP_WallSpline.BP_WallSpline_C|SetParent _returnvalue_3 _array_element_2)
                  (else
                    (bind _returnvalue_4 (Game|SpawnActorfromClass (Variables|Default|GetWallClass) (Math|Transform|MakeTransform (Default|GetEnd _array_element_2) "0, 0, 0" "1,1,1") "Undefined" _self (Math|Vector|MakeVector (Math|Float|SelectFloat 1.0 -1.0 (Math|Random|RandomBool)) 0.0 0.0) (Variables|Default|GetSpline%20Increment%20Amount) (Variables|Default|GetMin%20Wall%20Length) 0))
                    (Transformation|SetActorRotation _returnvalue_4 (Math|Conversions|RotationFromXVector (Variables|/Game/BP_WallSpline.BP_WallSpline_C|GetDirectionVector _returnvalue_4)))
                    (Utilities|Array|Add (Variables|Default|GetNew%20Paths) _returnvalue_4)
                    (Variables|/Game/BP_WallSpline.BP_WallSpline_C|SetParent _returnvalue_4 _array_element_2)))
                (Variables|/Game/BP_WallSpline.BP_WallSpline_C|SetSpawned _array_element_2 true))))))
      ;[1 1 1] Update all paths, and kill any paths exceeding the bounds
      (Variables|Default|SetStop true)
      (for _array_element_3 (Variables|Default|GetPaths)
        (Utilities|IsValid _array_element_3
          (:Is%20Valid
            (Default|Update _array_element_3)
            (if (Math|Boolean|ORBoolean (< (.x (Default|GetEnd _array_element_3)) (- (.x _returnvalue) _returnvalue_2)) (> (.x (Default|GetEnd _array_element_3)) (+ (.x _returnvalue) _returnvalue_2)) (< (.y (Default|GetEnd _array_element_3)) (- (.y _returnvalue) _returnvalue_2)) (> (.y (Default|GetEnd _array_element_3)) (+ (.y _returnvalue) _returnvalue_2)))
              (Default|SetDead _array_element_3)
              (elif (not (Variables|/Game/BP_WallSpline.BP_WallSpline_C|GetDead _array_element_3))
                (Variables|Default|SetStop false))))))
      ;[1 1 1] If at runtime, send event dispatchers etc.
      (if (Utilities|Time|IsValidTimerHandle (Variables|Default|GetUpdateTimer))
        (if (Variables|Default|GetStop)
          (Utilities|Time|ClearandInvalidateTimerbyHandle (Variables|Default|GetUpdateTimer))
          (Default|CallGenerated))))))

(event Custom|ThankYou!%20%28Click%29
  ;[1 1 1] THANK YOU
  (Effects|SpawnEmitteratLocation "/Game/ThankYou/PS_ThankYou.PS_ThankYou" (Transformation|GetActorLocation)))

(fn ConstructionScript)

(fn CalculateProbability
  (params (Length :type Float%20%28single-precision%29) (Multiplier :type Float%20%28single-precision%29))
  (return (Math|Float|Min(Float) (* (- (Math|Float|Power 2.0 (* Length (Variables|Default|GetExponent%20Multiplier) Multiplier)) 1.0) (Variables|Default|GetBaseProbability)) (Variables|Default|GetMax%20Probability))))